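; Boss enemy actor that hosts area, laser and slash attack shooter points and takes damage from player bullets.
; Each Tick copies shooter transforms to GameModeBoss, counter-rotates the laser and area rigs, and faces the player during slash attacks.
; GameModeBoss's start flag enables collision and triggers the BossAnimBP intro state.
; Once started, hits flag the animation, player bullets reduce game-mode health, and zero health sets Death and disables collision.
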(event Collision|EventHit
  (params (MyComp :type Primitive%20Component%20Object%20Reference) (Other :type Actor%20Object%20Reference) (OtherComp :type Primitive%20Component%20Object%20Reference) (bSelfMoved :type Boolean) (HitLocation :type Vector :default "0, 0, 0") (HitNormal :type Vector :default "0, 0, 0") (NormalImpulse :type Vector :default "0, 0, 0") (Hit :type Hit%20Result%20Structure%20%28by%20ref%29))
  ;[1 0.6845 0.3939] On-Bullet Hit
  (if (Variables|Default|GetstartBoss)
    (bind _asboss_anim_bp (Utilities|Casting|CastToBossAnimBP (Components|SkeletalMesh|GetAnimInstance (Variables|Character|GetMesh))))
    (if (not (Variables|/Game/Blueprints/BossAnimBP.BossAnimBP_C|Getdeath _asboss_anim_bp))
      (Variables|/Game/Blueprints/BossAnimBP.BossAnimBP_C|SetisHit _asboss_anim_bp true)
      (if (Actor|ActorHasTag Other "BulletPlayer")
        (bind _asbp_buller_player (Utilities|Casting|CastToBp_BullerPlayer Other))
        (Actor|DestroyActor _asbp_buller_player)
        (bind _asgame_mode_boss (Utilities|Casting|CastToGameModeBoss (Game|GetGameMode)))
        (Variables|/Game/Blueprints/GameModeBoss.GameModeBoss_C|SetBossHealth _asgame_mode_boss (- (Variables|/Game/Blueprints/GameModeBoss.GameModeBoss_C|GetBossHealth _asgame_mode_boss) (Variables|Default|GetBulletDamage)))
        (if (<= (Variables|/Game/Blueprints/GameModeBoss.GameModeBoss_C|GetBossHealth _asgame_mode_boss) 0.0)
          (Variables|/Game/Blueprints/BossAnimBP.BossAnimBP_C|Setdeath _asboss_anim_bp true)
          (Collision|SetActorEnableCollision false))
        (elif (not (Actor|ActorHasTag Other "Player"))
          (Actor|DestroyActor Other))))
    (elif (Actor|ActorHasTag Other "BulletPlayer")
      (bind _asbp_buller_player_2 (Utilities|Casting|CastToBp_BullerPlayer Other))
      (Actor|DestroyActor _asbp_buller_player_2))))

(event EventBeginPlay
  ;[0.2227 0.4517 0.7135] Set Collision Disabled at Start
  (Collision|SetActorEnableCollision false))

(event EventTick
  (params (DeltaSeconds :type Float%20%28single-precision%29))
  ;[0.4354 1 0.506] Settings
  ;;[1 0.2656 0.2656] Set Positions Area/Slash/Laser Attack
  (bind _asgame_mode_boss (Utilities|Casting|CastToGameModeBoss (Game|GetGameMode)))
  (Variables|/Game/Blueprints/GameModeBoss.GameModeBoss_C|SetlaserAtkNWPos _asgame_mode_boss (Transformation|GetWorldTransform (Variables|Default|GetLANorthWestShooter)))
  (Variables|/Game/Blueprints/GameModeBoss.GameModeBoss_C|SetlaserAtkSWPos _asgame_mode_boss (Transformation|GetWorldTransform (Variables|Default|GetLASouthWestShooter)))
  (Variables|/Game/Blueprints/GameModeBoss.GameModeBoss_C|SetlaserAtkSEPos _asgame_mode_boss (Transformation|GetWorldTransform (Variables|Default|GetLASouthEastShooter)))
  (Variables|/Game/Blueprints/GameModeBoss.GameModeBoss_C|SetslashAtkLeftPos _asgame_mode_boss (Transformation|GetWorldTransform (Variables|Default|GetSALeft3)))
  (Variables|/Game/Blueprints/GameModeBoss.GameModeBoss_C|SetslashAtkRightPos _asgame_mode_boss (Transformation|GetWorldTransform (Variables|Default|GetSARight3)))
  (Variables|/Game/Blueprints/GameModeBoss.GameModeBoss_C|SetlaserAtkNEPos _asgame_mode_boss (Transformation|GetWorldTransform (Variables|Default|GetLANorthEastShooter)))
  (Variables|/Game/Blueprints/GameModeBoss.GameModeBoss_C|SetareaAtkFrontPos _asgame_mode_boss (Transformation|GetWorldTransform (Variables|Default|GetAAFrontShooter)))
  (Variables|/Game/Blueprints/GameModeBoss.GameModeBoss_C|SetareaAtkBackPos _asgame_mode_boss (Transformation|GetWorldTransform (Variables|Default|GetAABackShooter)))
  (Variables|/Game/Blueprints/GameModeBoss.GameModeBoss_C|SetareaAtkLeftPos _asgame_mode_boss (Transformation|GetWorldTransform (Variables|Default|GetAALeftShooter)))
  (Variables|/Game/Blueprints/GameModeBoss.GameModeBoss_C|SetareaAtkRightPos _asgame_mode_boss (Transformation|GetWorldTransform (Variables|Default|GetAARightShooter)))
  (Variables|/Game/Blueprints/GameModeBoss.GameModeBoss_C|SetslashAtkPos _asgame_mode_boss (Transformation|GetWorldTransform (Variables|Default|GetSlashAttack)))
  (Transformation|AddLocalRotation (Variables|Default|GetLaserAttack) (Math|Rotator|MakeRotator 0.0 0.0 (* (* DeltaSeconds (Variables|Default|GetrotationSpeed)) -1.0)) false false)
  ;;[1 0.2656 0.2656] Rotate Area Attack
  (Transformation|AddLocalRotation (Variables|Default|GetAreaAttack) (Math|Rotator|MakeRotator 0.0 0.0 (* DeltaSeconds (Variables|Default|GetrotationSpeed))) false false)
  ;;[1 0.2656 0.2656] Start Boss Battle
  (if (Variables|/Game/Blueprints/GameModeBoss.GameModeBoss_C|GetstartBossMode _asgame_mode_boss)
    (Variables|Default|SetstartBoss (Variables|/Game/Blueprints/GameModeBoss.GameModeBoss_C|GetstartBossMode _asgame_mode_boss))
    (bind _asboss_anim_bp (Utilities|Casting|CastToBossAnimBP (Components|SkeletalMesh|GetAnimInstance (Variables|Character|GetMesh))))
    (bind _output_get (Variables|/Game/Blueprints/BossAnimBP.BossAnimBP_C|SetstartBoss _asboss_anim_bp (Variables|/Game/Blueprints/GameModeBoss.GameModeBoss_C|GetstartBossMode _asgame_mode_boss)))
    (if _output_get
      (Collision|SetActorEnableCollision true)
      (Utilities|FlowControl|Delay 0.1)
      (Variables|/Game/Blueprints/BossAnimBP.BossAnimBP_C|SetstartBoss _asboss_anim_bp false)
      (if (Variables|/Game/Blueprints/GameModeBoss.GameModeBoss_C|GetrealizeSlashAttack _asgame_mode_boss)
        ;[1 0.2656 0.2656] Boss Faces the Player
        (Transformation|SetActorRotation (Components|GetOwner (Variables|Character|GetMesh)) (Math|Conversions|RotationFromXVector (Math|Vector|RotateVector (Math|Vector|Normalize (* (- (Transformation|GetActorLocation (Game|Player|GetPlayerPawn 0)) (Transformation|GetActorLocation)) "1.000000,1.000000, 0")) "0, 0, 0")) :!label _label))
      (elif (Variables|/Game/Blueprints/GameModeBoss.GameModeBoss_C|GetrealizeSlashAttack _asgame_mode_boss)
        (goto _label)))))

(fn ConstructionScript)